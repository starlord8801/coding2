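; Base enemy character that exposes combat, aggro, movement speed and patrol actions.
; Attack plays a wheel kick montage and fires AttackFinished whether it completes or is interrupted.
; Gaining aggro swaps the mesh to a flat black material and sets the Aggroed flag, while losing it restores the material cached at BeginPlay.
; GetNextPatrolPointLocation steps along the PatrolRoute spline's points, reversing direction at either end to ping-pong.
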(event Custom|attack
  (Development|PrintString "attacking player")
  (Animation|Montage|PlayMontage (Variables|Character|GetMesh) "/Game/CloseCombatAnimSet/Animations/RootMotion/Attacks/NinjaWheelKick_MontageRM.NinjaWheelKick_MontageRM"
    (:OnCompleted
      _)
    (:OnInterrupted
      _))
  (Default|CallAttackFinished))

(event Custom|lose%20aggro
  (Rendering|Material|SetMaterial (Variables|Character|GetMesh) 0 (Variables|Default|GetoriginalMaterial))
  (Variables|Default|Setaggroed false))

(event Custom|get%20aggro
  (Rendering|Material|SetMaterial (Variables|Character|GetMesh) 0 "/Game/Materials/MI_FlatBlack.MI_FlatBlack")
  (Variables|Default|Setaggroed true))

(event Custom|set%20walk%20speed
  (params (new%20speed :type Float%20%28double-precision%29))
  (Variables|/Script/Engine.CharacterMovementComponent|SetMaxWalkSpeed (Variables|Character|GetCharacterMovement) new%20speed))

(event EventBeginPlay
  ;[0.15 0.15 0.15 0.5] set original mesh
  (Variables|Default|SetoriginalMaterial (Rendering|Material|GetMaterial (Variables|Character|GetMesh) 0)))

(fn ConstructionScript)

(fn GetNextPatrolPointLocation
  (Variables|patrol|SetPatrolPointIndex (+ (Variables|patrol|GetPatrolPointIndex) (Variables|patrol|GetpatrolRouteDirection)))
  (if (or (>= (Variables|patrol|GetPatrolPointIndex) (- (Spline|GetNumberOfSplinePoints (Variables|/Game/AI_Blueprints/bp_patrolRoute.bp_patrolRoute_C|GetSpline (Variables|patrol|GetpatrolRoute))) 1)) (<= (Variables|patrol|GetPatrolPointIndex) 0))
    (Variables|patrol|SetpatrolRouteDirection (* (Variables|patrol|GetpatrolRouteDirection) -1)) ; flip Direction
  )
  (return (Spline|GetLocationatSplinePoint (Variables|/Game/AI_Blueprints/bp_patrolRoute.bp_patrolRoute_C|GetSpline (Variables|patrol|GetpatrolRoute)) (Variables|patrol|GetPatrolPointIndex) "World")))