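; A key-gated door Blueprint that opens by sliding its mesh vertically when a player with a key approaches.
; A sphere overlap casts the other actor to BP_ThirdPersonCharacter and checks that its TotalKeys count is above zero.
; If so, a Timeline lerps the Door's relative Z downward; otherwise it prints that a key is needed.
; Keys are not consumed and the door has no closing logic.
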(event OnComponentBeginOverlap(Sphere)
  (params (OverlappedComponent :type Primitive%20Component%20Object%20Reference) (OtherActor :type Actor%20Object%20Reference) (OtherComp :type Primitive%20Component%20Object%20Reference) (OtherBodyIndex :type Integer) (bFromSweep :type Boolean) (SweepResult :type Hit%20Result%20Structure%20%28by%20ref%29))
  (Development|PrintString "something ran into me")
  (bind _asbp_third_person_character (Utilities|Casting|CastToBP_ThirdPersonCharacter OtherActor))
  (Development|PrintString "the player is at the door")
  (if (> (Variables|/Game/ThirdPerson/Blueprints/BP_ThirdPersonCharacter.BP_ThirdPersonCharacter_C|GettotalKeys _asbp_third_person_character) 0)
    (Development|PrintString "opening door" true true "(R=0.140164,G=1.000000,B=0.000000,A=1.000000)")
    (bind _newtrack_0 (Timeline|Timeline Play)
      (:Update
        (Transformation|SetRelativeLocation (Variables|Default|Getdoor) (Math|Vector|MakeVector 0.0 0.0 (Math|Float|Lerp 1.5e+02 -1.4e+02 _newtrack_0)) false false)))
    (else
      (Development|PrintString "you need a key" true true "(R=1.000000,G=0.000000,B=0.064205,A=1.000000)"))))

(event EventBeginPlay
  (Development|PrintString "door exists"))

(fn ConstructionScript)