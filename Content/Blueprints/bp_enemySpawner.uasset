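; Enemy spawner that populates the level with AI characters when play begins.
; It finds every Bp_enemySpawnPoint actor and gives each a 50% chance to spawn a BP_AiMoveTo at its transform.
; Each spawned AI receives a fixed name label, the Manny skeletal mesh and pink and blue flat materials.
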(event EventBeginPlay
  (Development|PrintString "enemy spawner is active")
  (bind _outactors (Actor|GetAllActorsOfClass "/Game/Blueprints/bp_enemySpawnPoint.bp_enemySpawnPoint_C"))
  (for _array_element _outactors
    (if (Math|Random|RandomBoolwithWeight 0.5)
      (bind _returnvalue (Game|SpawnActorfromClass "/Game/AI_Blueprints/BP_AiMoveTo.BP_AiMoveTo_C" (Transformation|GetActorTransform _array_element) "Undefined" "MultiplyWithRoot" 0 0))
      (Rendering|Components|TextRender|SetText (Variables|/Game/AI_Blueprints/BP_AiMoveTo.BP_AiMoveTo_C|GetaiNameText _returnvalue) (Utilities|Text|MakeLiteralText "MC CLAP YO HANDZ"))
      (Components|SkeletalMesh|SetSkeletalMeshAsset (Variables|/Script/Engine.Character|GetMesh _returnvalue) "/Game/Characters/Mannequins/Meshes/SKM_Manny.SKM_Manny")
      (Rendering|Material|SetMaterial (Variables|/Script/Engine.Character|GetMesh _returnvalue) 0 "/Game/Materials/MI_FlatPink.MI_FlatPink")
      (Rendering|Material|SetMaterial (Variables|/Script/Engine.Character|GetMesh _returnvalue) 1 "/Game/Materials/MI_FlatBlue.MI_FlatBlue"))))

(fn ConstructionScript)