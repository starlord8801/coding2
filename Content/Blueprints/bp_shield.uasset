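; Shield item actor that can be picked up, used and dropped, with debug text on pickup and use.
; Pickup snaps it to the hand_r socket of the given skeletal mesh and disables collision.
; Drop detaches it and restores collision, simulating physics for a brief delay before switching physics off.
; Primary use makes the shield visible, while secondary use only prints a message.
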(event EventPickup
  (params (skeletalMesh :type Skeletal%20Mesh%20Component%20Object%20Reference))
  (Development|PrintText (Utilities|Text|FormatText "{name} is getting picked up and attached to {mesh}" (Utilities|String|MakeLiteralString "shield")) true true "(R=0.984729,G=0.000000,B=1.000000,A=1.000000)" 6.0)
  (Transformation|AttachComponentToComponent skeletalMesh "hand_r" "SnapToTarget" "SnapToTarget" "SnapToTarget" true)
  (Collision|SetCollisionEnabled (Variables|Default|Getshield) "NoCollision"))

(event EventUsePrimary
  (Rendering|SetVisibility (Variables|Default|Getshield) true true)
  (Development|PrintText "shield on" true true "(R=1.000000,G=0.020616,B=0.000000,A=1.000000)" 6.0))

(event EventDrop
  (bind _shield (Variables|Default|Getshield))
  (Transformation|DetachFromActor "KeepWorld" "KeepWorld" "KeepWorld")
  (Physics|SetSimulatePhysics _shield true)
  (Collision|SetCollisionEnabled _shield "QueryAndPhysics")
  (Utilities|FlowControl|Delay 2.0)
  (Physics|SetSimulatePhysics _shield false))

(event EventUseSecondary
  (Development|PrintText "shield down" true true "(R=1.000000,G=0.020616,B=0.000000,A=1.000000)" 6.0))

(fn ConstructionScript)