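; GM_savLoad is a game mode that handles saving and loading player stats through an SG_playerStats save object.
; On BeginPlay it loads the PlayerSave slot and copies Stamina to the BP_ThirdPersonCharacter, or creates a fresh save object if none exists.
; The saveplayerstats event writes the held save object to that slot as it stands, without reading values from the character.
; Both paths print debug messages.
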(event Custom|Load%20Player%20Stats
  (bind _returnvalue (SaveGame|DoesSaveGameExist "PlayerSave"))
  (if _returnvalue
    (bind _returnvalue_2 (SaveGame|LoadGamefromSlot "PlayerSave"))
    (bind _assg_player_stats (Utilities|Casting|CastToSG_playerStats _returnvalue_2))
    (Variables|Default|SetSG_playerStats _assg_player_stats)
    (bind _asbp_third_person_character (Utilities|Casting|CastToBP_ThirdPersonCharacter (Game|GetPlayerCharacter 0)))
    (Variables|/Game/ThirdPerson/Blueprints/BP_ThirdPersonCharacter.BP_ThirdPersonCharacter_C|SetStamina _asbp_third_person_character (Variables|/Game/Blueprints/savingLoading/SG_playerStats.SG_playerStats_C|Getstamina (Variables|Default|GetSG_playerStats)))
    (Development|PrintString "Player stats have been loaded" true true "(R=1.000000,G=0.198919,B=0.000000,A=1.000000)" 8.0)
    (else
      (bind _returnvalue_3 (SaveGame|CreateSaveGameObject "/Game/Blueprints/savingLoading/SG_playerStats.SG_playerStats_C"))
      (Variables|Default|SetSG_playerStats _returnvalue_3))))

(event Custom|save%20player%20stats
  (bind _returnvalue (SaveGame|SaveGametoSlot (Variables|Default|GetSG_playerStats) "PlayerSave"))
  (if _returnvalue
    (Development|PrintText "Player Stats written to save game file" true true "(R=0.063372,G=1.000000,B=0.000000,A=1.000000)")
    (else
      (Development|PrintText "Player Stats could not be written to save game file" true true "(R=1.000000,G=0.000000,B=0.029186,A=1.000000)"))))

(event EventBeginPlay
  (Development|PrintString "Loading the savLoad game mode" true true "(R=1.000000,G=0.250437,B=0.000000,A=1.000000)" 1e+01)
  (CallFunction|LoadPlayerStats))

(fn ConstructionScript)