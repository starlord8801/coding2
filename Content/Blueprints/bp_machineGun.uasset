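; Machine gun weapon Blueprint that can be picked up, used and dropped, with its firing still a debug-print placeholder.
; Pickup prints a debug message, snaps the gun to the hand_r socket of the given skeletal mesh and disables body collision.
; Drop detaches it in world space, restores collision and briefly simulates physics before switching simulation off after a delay.
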(event EventBeginPlay)

(event EventPickup
  (params (skeletalMesh :type Skeletal%20Mesh%20Component%20Object%20Reference))
  (Development|PrintText (Utilities|Text|FormatText "{name} is getting picked up and attached to {mesh}" (Utilities|String|MakeLiteralString "Machine Gun") skeletalMesh) true true "(R=0.984729,G=0.000000,B=1.000000,A=1.000000)" 6.0)
  (Transformation|AttachComponentToComponent skeletalMesh "hand_r" "SnapToTarget" "SnapToTarget" "SnapToTarget" true)
  (Collision|SetCollisionEnabled (Variables|Default|GetmachineGunBody) "NoCollision"))

(event EventUsePrimary
  (Development|PrintText "Pew Pew Pew" true true "(R=1.000000,G=0.020616,B=0.000000,A=1.000000)" 6.0))

(event EventDrop
  (bind _machinegunbody (Variables|Default|GetmachineGunBody))
  (Transformation|DetachFromActor "KeepWorld" "KeepWorld" "KeepWorld")
  (Physics|SetSimulatePhysics _machinegunbody true)
  (Collision|SetCollisionEnabled _machinegunbody "QueryAndPhysics")
  (Utilities|FlowControl|Delay 2.0)
  (Physics|SetSimulatePhysics _machinegunbody false))

(fn ConstructionScript)