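; Test Blueprint that exercises loops and arrays by repeatedly printing debug messages in random colors.
; BeginPlay starts DelayLoop, a self-calling event that prints an incrementing counter, waits one second, runs PrintColors, then repeats indefinitely.
; PrintColors shuffles the TextColors array and loops over it, printing a randomly picked color and index per iteration rather than the current element, then a completion message.
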(event Custom|delay%20loop
  (Development|PrintString (Utilities|String|Append "starting delay loop # " (Utilities|String|ToString(Integer) (Variables|Default|GetdelayLoopCounter))))
  (Math|Integer|IncrementInt (Variables|Default|GetdelayLoopCounter)
    (:%20%20
      (Utilities|FlowControl|Delay 1.0)
      (CallFunction|PrintColors)
      (CallFunction|DelayLoop))))

(event Custom|print%20colors
  (bind _array (Utilities|Array|MakeArray "(R=1.000000,G=0.010928,B=0.000000,A=1.000000)" "(R=0.370960,G=1.000000,B=0.000000,A=1.000000)" "(R=0.038699,G=0.000184,B=1.000000,A=1.000000)" "(R=1.000000,G=0.919441,B=0.000000,A=1.000000)" ""))
  (bind _textcolors (Variables|Default|GettextColors))
  (bind (_outitem _outindex) (Utilities|Array|Random _array))
  (Utilities|Array|Shuffle _textcolors)
  (for _array_element _textcolors
    (Development|PrintString (Utilities|String|Append "printing color #" (Utilities|String|ToString(Integer) _outindex)) true true _outitem))
  (Development|PrintString "we are done printing color" true true "(R=0.000000,G=0.000000,B=0.000000,A=1.000000)"))

(event EventBeginPlay
  (Development|PrintString "loops and lists is active")
  (CallFunction|DelayLoop))

(fn ConstructionScript)