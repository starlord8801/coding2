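; An elemental barrier actor that kills any player character lacking immunity to its element.
; On BeginPlay, a text render labels the barrier by its ElementalType.
; When a BP_ThirdPersonCharacter overlaps the cube, its ElementalImmunity is compared with the barrier's type.
; A mismatch prints a death message and quits the game after a short delay.
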(event OnComponentBeginOverlap(cube)
  (params (OverlappedComponent :type Primitive%20Component%20Object%20Reference) (OtherActor :type Actor%20Object%20Reference) (OtherComp :type Primitive%20Component%20Object%20Reference) (OtherBodyIndex :type Integer) (bFromSweep :type Boolean) (SweepResult :type Hit%20Result%20Structure%20%28by%20ref%29))
  (bind _asbp_third_person_character (Utilities|Casting|CastToBP_ThirdPersonCharacter OtherActor))
  (if (not (Utilities|Enum|Equal(Enum) (Variables|Default|GetelementalType) (Variables|/Game/ThirdPerson/Blueprints/BP_ThirdPersonCharacter.BP_ThirdPersonCharacter_C|GetelementalImmunity _asbp_third_person_character)))
    (Development|PrintString "you're dead")
    (Utilities|FlowControl|Delay 2.0)
    (Game|QuitGame 0 "Quit" false)))

(event EventBeginPlay
  (switch Utilities|FlowControl|Switch|SwitchonelementalType (Variables|Default|GetelementalType)
    (:NewEnumerator1
      (Rendering|Components|TextRender|SetText (Variables|Default|GetTextRender) (Utilities|Text|MakeLiteralText "Barrier of Fire")))
    (:NewEnumerator2
      (Rendering|Components|TextRender|SetText (Variables|Default|GetTextRender) (Utilities|Text|MakeLiteralText "Barrier of water")))
    (:NewEnumerator3
      (Rendering|Components|TextRender|SetText (Variables|Default|GetTextRender) (Utilities|Text|MakeLiteralText "Barrier of earth")))
    (:NewEnumerator4
      (Rendering|Components|TextRender|SetText (Variables|Default|GetTextRender) (Utilities|Text|MakeLiteralText "Barrier of air")))
    (:NewEnumerator5
      (Rendering|Components|TextRender|SetText (Variables|Default|GetTextRender) (Utilities|Text|MakeLiteralText "Barrier of posion")))
    (:NewEnumerator6
      (Rendering|Components|TextRender|SetText (Variables|Default|GetTextRender) (Utilities|Text|MakeLiteralText "Barrier of void")))))

(fn ConstructionScript)